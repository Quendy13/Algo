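; Pawn Blueprint that measures how many actions per minute the player makes with the E key.
; Each E press increments an action counter and prints a default debug message.
; Tick accumulates elapsed time and prints the running actions-per-minute average every frame.
; An unconnected string assignment and substring node remain in the graph but never run.
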(event EventTick
  (params (DeltaSeconds :type Float%20%28single-precision%29))
  (Variables|Default|SetSeconds (+ DeltaSeconds (Variables|Default|GetSeconds)))
  (Development|PrintString (Utilities|String|ToString(Float) (/ (Variables|Default|GetAction) (/ (Variables|Default|GetSeconds) 6e+01)))))

(event Input|KeyboardEvents|E
  (params (Key :type Key%20Structure :default "None"))
  (:Pressed
    (Math|Integer|IncrementInt (Variables|Default|GetAction)
      (:%20%20
        (Development|PrintString "Hello")))))

(fn ConstructionScript)