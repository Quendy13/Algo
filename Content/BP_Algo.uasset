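; BP_Algo is a small Blueprint that calculates and prints the average (Moyenne) of its Notes array when play begins.
; BeginPlay calls MoyenneFunction, which loops over the array indices, accumulates each value into Moyenne and divides by the array length.
; The result is converted to text, then to a string, and shown with PrintString.
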(event EventBeginPlay
  (CallFunction|MoyenneFunction))

(fn ConstructionScript)

(fn MoyenneFunction
  (bind _notes (Variables|Default|GetNotes))
  (for _index (range 0 (Utilities|Array|LastIndex _notes))
    (Variables|Default|SetMoyenne (+ (Utilities|Array|Get(acopy) _notes _index) (Variables|Default|GetMoyenne))))
  (Variables|Default|SetMoyenne (/ (Variables|Default|GetMoyenne) (Utilities|Array|Length _notes)))
  (Development|PrintString (Utilities|String|ToString(Text) (Utilities|Text|ToText(Float) (Variables|Default|GetMoyenne) "HalfToEven" false true 1 324 0 2))))